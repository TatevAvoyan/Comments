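; An actor whose point light continually fades between random colors.
; On BeginPlay it picks a random RGB target, and the ColorAnimation timeline interpolates the light from the current color toward it.
; When the timeline finishes, the target becomes the new start color and the cycle restarts with another random target, looping indefinitely.
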(event EventBeginPlay
  (Variables|Default|SetColor2 (Utilities|Struct|MakeLinearColor (Math|Random|RandomFloat) (Math|Random|RandomFloat) (Math|Random|RandomFloat) 0.0) :!label _label)
  (bind _newtrack_0 (Timeline|ColorAnimation PlayFromStart)
    (:Update
      (Rendering|Components|Light|SetLightColor (Variables|Default|GetPointLight) (Math|Color|Lerp(LinearColor) (Variables|Default|GetColor1) (Variables|Default|GetColor2) _newtrack_0) true))
    (:Finished
      (Variables|Default|SetColor1 (Variables|Default|GetColor2))
      (goto _label))))

(fn ConstructionScript)